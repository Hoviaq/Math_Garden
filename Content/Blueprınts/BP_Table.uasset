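; BP_Table is a pickup table that holds one basket at a time for the player farmer to take.
; FunctionBasketSpawner shows the given basket mesh on the table when it is empty.
; FarmInteraction hides it, copies the mesh onto BP_Farmer's basket component and flags the farmer as carrying.
; Both mirror the table's CanTake state into GM_Farmer's Istake flag through a game mode reference cached on BeginPlay.
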(event EventBeginPlay
  (bind _asgm_farmer (Utilities|Casting|CastToGM_Farmer (Game|GetGameMode)))
  (Variables|Default|SetAs%20GM%20Farmer _asgm_farmer))

(event Collision|EventActorBeginOverlap
  (params (OtherActor :type Actor%20Object%20Reference)))

(event EventTick
  (params (DeltaSeconds :type Float%20%28single-precision%29)))

(event EventFunctionBasketSpawner
  (params (Basket_Type :type Static%20Mesh%20Object%20Reference))
  (bind _sm_normal_basket (Variables|Default|GetSM_Normal_Basket))
  (if (not (Variables|Default|GetCanTake))
    (Components|StaticMesh|SetStaticMesh _sm_normal_basket Basket_Type)
    (Rendering|SetVisibility _sm_normal_basket true false)
    (bind _output_get (Variables|Default|SetCanTake true))
    (Variables|/Game/Blueprınts/Character/GM_Farmer.GM_Farmer_C|SetIstake? (Variables|Default|GetAs%20GM%20Farmer) _output_get)))

(event EventFarmInteraction
  (if (Variables|Default|GetCanTake)
    (Rendering|SetVisibility (Variables|Default|GetSM_Normal_Basket) false false)
    (bind _asbp_farmer (Utilities|Casting|CastToBP_Farmer (Game|Player|GetPlayerPawn 0)))
    (Components|StaticMesh|SetStaticMesh (Variables|/Game/Blueprınts/Character/BP_Farmer.BP_Farmer_C|GetSM_Normal_Basket _asbp_farmer) (Variables|/Script/Engine.StaticMeshComponent|GetStaticMesh (Variables|Default|GetSM_Normal_Basket)))
    (Rendering|SetVisibility (Variables|/Game/Blueprınts/Character/BP_Farmer.BP_Farmer_C|GetSM_Normal_Basket _asbp_farmer) true false)
    (bind _output_get (Variables|Default|SetCanTake false))
    (Variables|/Game/Blueprınts/Character/GM_Farmer.GM_Farmer_C|SetIstake? (Variables|Default|GetAs%20GM%20Farmer) _output_get)
    (Variables|/Game/Blueprınts/Character/BP_Farmer.BP_Farmer_C|SetIsCarrying? _asbp_farmer true)))

(fn ConstructionScript)