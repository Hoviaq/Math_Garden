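; Function library that generates random arithmetic questions, apparently for a math game with fruit icons.
; Each function returns two random operands, their result, an operator symbol and a random icon from the Texture array.
; Addition, subtraction and multiplication come in basic and regular variants with different ranges, with subtraction deriving its second operand's range from the first.
; Basic division is unfinished, returning a zero result and a multiplication symbol.
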(fn AddfuncBasic
  (bind _returnvalue (Math|Random|RandomIntegerinRange 1 25))
  (bind _returnvalue_2 (Math|Random|RandomIntegerinRange 1 25))
  (return (+ _returnvalue _returnvalue_2) _returnvalue _returnvalue_2 "+" (.OutItem (Utilities|Array|Random (LocalVariables|Gettexture)))))

(fn Addfunc
  (bind _returnvalue (Math|Random|RandomIntegerinRange 25 50))
  (bind _returnvalue_2 (Math|Random|RandomIntegerinRange 25 50))
  (return (+ _returnvalue_2 _returnvalue) _returnvalue_2 _returnvalue "+" (.OutItem (Utilities|Array|Random (LocalVariables|Gettexture)))))

(fn Subfunc
  (bind _returnvalue (Math|Random|RandomIntegerinRange 50 100))
  (bind _returnvalue_2 (- _returnvalue 40))
  (bind _returnvalue_3 (+ _returnvalue -15))
  (bind _returnvalue_4 (Math|Random|RandomIntegerinRange _returnvalue_2 _returnvalue_3))
  (return (- _returnvalue _returnvalue_4) _returnvalue _returnvalue_4 "-" (.OutItem (Utilities|Array|Random (LocalVariables|Gettexture)))))

(fn SubfuncBasic
  (bind _returnvalue (Math|Random|RandomIntegerinRange 5 50))
  (bind _returnvalue_2 (- _returnvalue -3))
  (bind _returnvalue_3 (Math|Random|RandomIntegerinRange 1 _returnvalue_2))
  (return (- _returnvalue _returnvalue_3) _returnvalue _returnvalue_3 "-" (.OutItem (Utilities|Array|Random (LocalVariables|Gettexture)))))

(fn MultifuncBasic
  (bind _returnvalue (Math|Random|RandomIntegerinRange 3 10))
  (bind _returnvalue_2 (Math|Random|RandomIntegerinRange 3 5))
  (return (* _returnvalue_2 _returnvalue) _returnvalue_2 _returnvalue "x" (.OutItem (Utilities|Array|Random (LocalVariables|Gettexture)))))

(fn Multifunc
  (bind _returnvalue (Math|Random|RandomIntegerinRange 3 10))
  (bind _returnvalue_2 (Math|Random|RandomIntegerinRange 3 10))
  (return (* _returnvalue_2 _returnvalue) _returnvalue_2 _returnvalue "x" (.OutItem (Utilities|Array|Random (LocalVariables|Gettexture)))))

(fn DivfuncBasic
  (return 0 (Math|Random|RandomIntegerinRange 3 5) (Math|Random|RandomIntegerinRange 3 10) "x" (.OutItem (Utilities|Array|Random (LocalVariables|Gettexture)))))