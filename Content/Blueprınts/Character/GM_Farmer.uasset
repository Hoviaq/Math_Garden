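; GM_Farmer is the game mode for a farming game, holding fruit counts and coins and checking the player's answers to NPCs.
; BeginPlay shows the main screen and loads or creates the save object, then autosaves every ten seconds; pear count loads from the saved peach value.
; A custom event compares input and fruit icon, shows an NPC speech bubble, pays coins when correct, and calls the NPC's deadline event.
; Another event messages the spawner.
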(event Custom|CustomEvent
  (if (== (Variables|Default|GetInput) (Variables|Default|GetResult))
    (if (Utilities|Enum|Equal(Enum) (Variables|Default|GetFruitIcon) (Variables|Default|GetFruitIcon_Char))
      (bind _asbp_npc (Utilities|Casting|CastToBP_NPC (Variables|Default|GetNPC_Ref)))
      (bind _returnvalue (UserInterface|CreateWidget "/Game/Blueprınts/Widget_Blueprints/WB_SpeechBubble1.WB_SpeechBubble1_C" 0 "Thank You Honey !!!"))
      (UserInterface|SetWidget (Variables|/Game/Blueprınts/NPC/BP_NPC.BP_NPC_C|GetWidget _asbp_npc) _returnvalue)
      (Variables|/Game/Blueprınts/NPC/BP_NPC.BP_NPC_C|SetResultCheck _asbp_npc true)
      (Utilities|FlowControl|Delay 1.5)
      (Default|EventDeadline _asbp_npc)
      (Development|PrintText "huhuuuu")
      (bind _output_get (Variables|Default|SetGain (* (Variables|Default|GetResult) 2)))
      (Variables|Default|SetCoin (+ (Variables|Default|GetCoin) _output_get))
      (Class|BPIFarm|FunctionGain(Message) (Variables|Default|GetWidgetRef) _output_get)
      (else
        (bind _asbp_npc_2 (Utilities|Casting|CastToBP_NPC (Variables|Default|GetNPC_Ref) :!label _label))
        (bind _returnvalue_2 (UserInterface|CreateWidget "/Game/Blueprınts/Widget_Blueprints/WB_SpeechBubble1.WB_SpeechBubble1_C" 0 "It is Wrong Honey !!!"))
        (UserInterface|SetWidget (Variables|/Game/Blueprınts/NPC/BP_NPC.BP_NPC_C|GetWidget _asbp_npc_2) _returnvalue_2)
        (Utilities|FlowControl|Delay 2.0)
        (Default|EventDeadline _asbp_npc_2)))
    (else
      (goto _label))))

(event Custom|CustomEvent_0
  (Class|BPIFarm|FunctionNPCSpawnerr(Message) (Variables|Default|GetSpawner)))

(event EventBeginPlay
  (bind _returnvalue (UserInterface|CreateWidget "/Game/Blueprınts/Widget_Blueprints/MainScree.MainScree_C"))
  (bind _output_get (Variables|Default|SetWidgetRef _returnvalue))
  (UserInterface|Viewport|AddtoViewport _output_get 0)
  (bind _returnvalue_2 (SaveGame|DoesSaveGameExist "GameMode"))
  (if _returnvalue_2
    (bind _returnvalue_3 (SaveGame|LoadGamefromSlot "GameMode"))
    (bind _assg_game_mode (Utilities|Casting|CastToSG_GameMode _returnvalue_3))
    (bind _output_get_2 (Variables|Default|SetSaveGame_GM _assg_game_mode))
    (Variables|Default|SetCurrentAppleAmount (Variables|/Game/Blueprınts/Character/SG_GameMode.SG_GameMode_C|GetCurrentAppleAmount _output_get_2))
    (Variables|Default|SetCurrentOrangeAmount (Variables|/Game/Blueprınts/Character/SG_GameMode.SG_GameMode_C|GetCurrentOrangeAmount _output_get_2))
    (Variables|Default|SetCurrentPearAmount (Variables|/Game/Blueprınts/Character/SG_GameMode.SG_GameMode_C|GetCurrentPeachAmount _output_get_2))
    (Variables|Default|SetCurrentPeachAmount (Variables|/Game/Blueprınts/Character/SG_GameMode.SG_GameMode_C|GetCurrentPeachAmount _output_get_2))
    (Variables|Default|SetCurrentPomagranteAmount (Variables|/Game/Blueprınts/Character/SG_GameMode.SG_GameMode_C|GetCurrentPomagranteAmount _output_get_2))
    (Variables|Default|SetCoin (Variables|/Game/Blueprınts/Character/SG_GameMode.SG_GameMode_C|GetCoin _output_get_2))
    (Utilities|Time|SetTimerbyFunctionName 0 "Save game" 1e+01 true)
    (else
      (bind _returnvalue_4 (SaveGame|CreateSaveGameObject "/Game/Blueprınts/Character/SG_GameMode.SG_GameMode_C"))
      (Variables|Default|SetSaveGame_GM _returnvalue_4)
      (Utilities|Time|SetTimerbyFunctionName 0 "Save game" 1e+01 true))))

(fn ConstructionScript)

(fn SaveGame
  (bind _savegame_gm (Variables|Default|GetSaveGame_GM))
  (Variables|/Game/Blueprınts/Character/SG_GameMode.SG_GameMode_C|SetCurrentAppleAmount _savegame_gm (Variables|Default|GetCurrentAppleAmount))
  (Variables|/Game/Blueprınts/Character/SG_GameMode.SG_GameMode_C|SetCurrentOrangeAmount _savegame_gm (Variables|Default|GetCurrentOrangeAmount))
  (Variables|/Game/Blueprınts/Character/SG_GameMode.SG_GameMode_C|SetCurrentPearAmount _savegame_gm (Variables|Default|GetCurrentPearAmount))
  (Variables|/Game/Blueprınts/Character/SG_GameMode.SG_GameMode_C|SetCurrentPeachAmount _savegame_gm (Variables|Default|GetCurrentPeachAmount))
  (Variables|/Game/Blueprınts/Character/SG_GameMode.SG_GameMode_C|SetCurrentPomagranteAmount _savegame_gm (Variables|Default|GetCurrentPomagranteAmount))
  (Variables|/Game/Blueprınts/Character/SG_GameMode.SG_GameMode_C|SetCoin _savegame_gm (Variables|Default|GetCoin))
  (SaveGame|SaveGametoSlot _savegame_gm "GameMode"))