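; BP_NPC_Take is an interaction Blueprint through which the player farmer hands a carried basket to an NPC.
; On FarmInteraction, if BP_Farmer is carrying, it turns off selection on GM_Farmer and fires the game mode's CustomEvent.
; It then sends the basket's static mesh to the game mode's referenced NPC via FunctionBasketSpawnerMessage and hides the farmer's basket, without clearing the carrying flag.
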(event EventBeginPlay)

(event Collision|EventActorBeginOverlap
  (params (OtherActor :type Actor%20Object%20Reference)))

(event EventTick
  (params (DeltaSeconds :type Float%20%28single-precision%29)))

(event EventFarmInteraction
  (bind _asbp_farmer (Utilities|Casting|CastToBP_Farmer (Game|Player|GetPlayerPawn 0)))
  (if (Variables|/Game/Blueprınts/Character/BP_Farmer.BP_Farmer_C|GetIsCarrying? _asbp_farmer)
    (bind _asgm_farmer (Utilities|Casting|CastToGM_Farmer (Game|GetGameMode)))
    (Variables|/Game/Blueprınts/Character/GM_Farmer.GM_Farmer_C|Setcanselect _asgm_farmer false)
    (Default|CustomEvent _asgm_farmer)
    (Class|BPIFarm|FunctionBasketSpawner(Message) (Variables|/Game/Blueprınts/Character/GM_Farmer.GM_Farmer_C|GetNPC_Ref _asgm_farmer) (Variables|/Script/Engine.StaticMeshComponent|GetStaticMesh (Variables|/Game/Blueprınts/Character/BP_Farmer.BP_Farmer_C|GetSM_Normal_Basket _asbp_farmer)))
    (Rendering|SetVisibility (Variables|/Game/Blueprınts/Character/BP_Farmer.BP_Farmer_C|GetSM_Normal_Basket _asbp_farmer) false false)))

(fn ConstructionScript)