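; NPC for a farmer math game that walks to a fixed spot, poses an arithmetic question, then leaves.
; On arrival, a timer calls the function named by GI_Farmer's Text, such as simple or hard add, subtract or multiply.
; These store the answer and fruit in GM_Farmer and show a speech bubble.
; After a fixed wait it clears the player's basket, walks away, notifies GM_Farmer and self-destructs; a separate event shows its carried basket.
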(event Custom|Event_GotoTarget
  (AI|AIMoveTo self "380.000000,286.000000,25.000000" 0 5.0 false
    (:OnSuccess
      (Utilities|Time|SetTimerbyFunctionName 0 (Utilities|String|ToString(Name) (Variables|/Game/Blueprınts/Character/GI_Farmer.GI_Farmer_C|Gettext (Variables|Default|GetAs%20GI%20Farmer))) 0.1)
      (Utilities|FlowControl|Delay 2e+01)
      (bind _asbp_farmer (Utilities|Casting|CastToBP_Farmer (Game|Player|GetPlayerPawn 0)))
      (Variables|/Game/Blueprınts/Character/BP_Farmer.BP_Farmer_C|SetIsCarrying? _asbp_farmer false)
      (Rendering|SetVisibility (Variables|/Game/Blueprınts/Character/BP_Farmer.BP_Farmer_C|GetSM_Normal_Basket _asbp_farmer) false false)
      (Rendering|SetVisibility (Variables|Default|GetWidget) false false)
      (CallFunction|EventDeadline))))

(event Custom|Event_Deadline
  (Rendering|SetVisibility (Variables|Default|GetWidget) false false)
  (AI|AIMoveTo self "-137.000000,-682.000000,10.000000" 0 5.0 false
    (:OnSuccess
      (bind _asgm_farmer (Utilities|Casting|CastToGM_Farmer (Game|GetGameMode)))
      (Default|CustomEvent0 _asgm_farmer)
      (Actor|DestroyActor))))

(event EventBeginPlay
  (CallFunction|EventGotoTarget)
  (bind _asgi_farmer (Utilities|Casting|CastToGI_Farmer (Game|GetGameInstance)))
  (bind _output_get (Variables|Default|SetAs%20GI%20Farmer _asgi_farmer)))

(event Collision|EventActorBeginOverlap
  (params (OtherActor :type Actor%20Object%20Reference)))

(event EventFunctionGain
  (params (Gain :type Float%20%28double-precision%29)))

(event EventFunctionBasketSpawner
  (params (Basket_Type :type Static%20Mesh%20Object%20Reference))
  (bind _sm_normal_basket (Variables|Default|GetSM_Normal_Basket))
  (if (Variables|Default|GetResultCheck)
    (Variables|Default|Setiscarry? true)
    (Components|StaticMesh|SetStaticMesh _sm_normal_basket Basket_Type)
    (Rendering|SetVisibility _sm_normal_basket true false)))

(fn ConstructionScript)

(fn Fun)

(fn FunctionSimpleAdd
  (bind _widget (Variables|Default|GetWidget))
  (bind (_result _first _second _islem _icon) (CallFunction|AddfuncBasic))
  (bind _asgm_farmer (Utilities|Casting|CastToGM_Farmer (Game|GetGameMode)))
  (Variables|/Game/Blueprınts/Character/GM_Farmer.GM_Farmer_C|SetResult _asgm_farmer _result)
  (Variables|/Game/Blueprınts/Character/GM_Farmer.GM_Farmer_C|SetFruitIcon _asgm_farmer (Utilities|GetObjectName _icon))
  (bind _returnvalue (UserInterface|CreateWidget "/Game/Blueprınts/Widget_Blueprints/WB_SpeechBubble.WB_SpeechBubble_C" 0 _first _second _islem _icon))
  (Rendering|SetVisibility _widget true false)
  (UserInterface|SetWidget _widget _returnvalue))

(fn FunctionHardAdd
  (bind _widget (Variables|Default|GetWidget))
  (bind (_result _first _second _newparam _fruiticon) (CallFunction|Addfunc))
  (bind _asgm_farmer (Utilities|Casting|CastToGM_Farmer (Game|GetGameMode)))
  (Variables|/Game/Blueprınts/Character/GM_Farmer.GM_Farmer_C|SetResult _asgm_farmer _result)
  (Variables|/Game/Blueprınts/Character/GM_Farmer.GM_Farmer_C|SetFruitIcon _asgm_farmer (Utilities|GetObjectName _fruiticon))
  (bind _returnvalue (UserInterface|CreateWidget "/Game/Blueprınts/Widget_Blueprints/WB_SpeechBubble.WB_SpeechBubble_C" 0 _first _second _newparam _fruiticon))
  (Rendering|SetVisibility _widget true false)
  (UserInterface|SetWidget _widget _returnvalue))

(fn FunctionSimpleSub
  (bind _widget (Variables|Default|GetWidget))
  (bind (_result _first _second _newparam _fruiticon) (CallFunction|SubfuncBasic))
  (bind _asgm_farmer (Utilities|Casting|CastToGM_Farmer (Game|GetGameMode)))
  (Variables|/Game/Blueprınts/Character/GM_Farmer.GM_Farmer_C|SetResult _asgm_farmer _result)
  (Variables|/Game/Blueprınts/Character/GM_Farmer.GM_Farmer_C|SetFruitIcon _asgm_farmer (Utilities|GetObjectName _fruiticon))
  (bind _returnvalue (UserInterface|CreateWidget "/Game/Blueprınts/Widget_Blueprints/WB_SpeechBubble.WB_SpeechBubble_C" 0 _first _second _newparam _fruiticon))
  (Rendering|SetVisibility _widget true false)
  (UserInterface|SetWidget _widget _returnvalue))

(fn FunctionHardSub
  (bind _widget (Variables|Default|GetWidget))
  (bind (_result _first _second _newparam _fruiticon) (CallFunction|Subfunc))
  (bind _asgm_farmer (Utilities|Casting|CastToGM_Farmer (Game|GetGameMode)))
  (Variables|/Game/Blueprınts/Character/GM_Farmer.GM_Farmer_C|SetResult _asgm_farmer _result)
  (Variables|/Game/Blueprınts/Character/GM_Farmer.GM_Farmer_C|SetFruitIcon _asgm_farmer (Utilities|GetObjectName _fruiticon))
  (bind _returnvalue (UserInterface|CreateWidget "/Game/Blueprınts/Widget_Blueprints/WB_SpeechBubble.WB_SpeechBubble_C" 0 _first _second _newparam _fruiticon))
  (Rendering|SetVisibility _widget true false)
  (UserInterface|SetWidget _widget _returnvalue))

(fn FunctionSimpleMulti
  (bind _widget (Variables|Default|GetWidget))
  (bind (_result _first _second _newparam _fruiticon) (CallFunction|MultifuncBasic))
  (bind _asgm_farmer (Utilities|Casting|CastToGM_Farmer (Game|GetGameMode)))
  (Variables|/Game/Blueprınts/Character/GM_Farmer.GM_Farmer_C|SetResult _asgm_farmer _result)
  (Variables|/Game/Blueprınts/Character/GM_Farmer.GM_Farmer_C|SetFruitIcon _asgm_farmer (Utilities|GetObjectName _fruiticon))
  (bind _returnvalue (UserInterface|CreateWidget "/Game/Blueprınts/Widget_Blueprints/WB_SpeechBubble.WB_SpeechBubble_C" 0 _first _second _newparam _fruiticon))
  (Rendering|SetVisibility _widget true false)
  (UserInterface|SetWidget _widget _returnvalue))

(fn FunctionHardMulti
  (bind _widget (Variables|Default|GetWidget))
  (bind (_result _first _second _newparam _fruiticon) (CallFunction|Multifunc))
  (bind _asgm_farmer (Utilities|Casting|CastToGM_Farmer (Game|GetGameMode)))
  (Variables|/Game/Blueprınts/Character/GM_Farmer.GM_Farmer_C|SetResult _asgm_farmer _result)
  (Variables|/Game/Blueprınts/Character/GM_Farmer.GM_Farmer_C|SetFruitIcon _asgm_farmer (Utilities|GetObjectName _fruiticon))
  (bind _returnvalue (UserInterface|CreateWidget "/Game/Blueprınts/Widget_Blueprints/WB_SpeechBubble.WB_SpeechBubble_C" 0 _first _second _newparam _fruiticon))
  (Rendering|SetVisibility _widget true false)
  (UserInterface|SetWidget _widget _returnvalue))