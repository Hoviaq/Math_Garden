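; BP_NPCSpawner spawns BP_NPC characters at its own location and ends the round once its spawn count passes ten.
; Each call to its spawner event, if CanSpawn is set, waits briefly, spawns an AI NPC and increments the count.
; The new NPC is stored on GM_Farmer and sent toward its target.
; Past the limit, the event pauses the game and shows the WB_Levels widget with the mouse cursor.
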(event EventBeginPlay)

(event Collision|EventActorBeginOverlap
  (params (OtherActor :type Actor%20Object%20Reference)))

(event EventTick
  (params (DeltaSeconds :type Float%20%28single-precision%29)))

(event EventFunctionNPCSpawnerr
  ;[1 1 1] Npcspawner Interaction
  (if (<= (Variables|Default|GetNPCvalue) 10)
    (if (Variables|Default|GetCanSpawn)
      (Utilities|FlowControl|Delay 2.0)
      (CallFunction|FunctionNPCSpawner)
      (Variables|Default|SetNPCvalue (+ (Variables|Default|GetNPCvalue) 1)))
    (else
      (Game|SetGamePaused true)
      (bind _returnvalue (UserInterface|CreateWidget "/Game/Blueprınts/Widget_Blueprints/WB_Levels.WB_Levels_C"))
      (UserInterface|Viewport|AddtoViewport _returnvalue 0)
      (Variables|/Script/Engine.PlayerController|SetbShowMouseCursor (Game|GetPlayerController 0) true))))

(fn ConstructionScript)

(fn FunctionNPCSpawner
  (bind _defaultsceneroot (Variables|Default|GetDefaultSceneRoot))
  (bind _returnvalue (AI|SpawnAIFromClass "/Game/Blueprınts/NPC/BP_NPC.BP_NPC_C" 0 (Transformation|GetWorldLocation _defaultsceneroot) (Transformation|GetWorldRotation _defaultsceneroot) false 0))
  (bind _asgm_farmer (Utilities|Casting|CastToGM_Farmer (Game|GetGameMode)))
  (Variables|/Game/Blueprınts/Character/GM_Farmer.GM_Farmer_C|SetNPC_Ref _asgm_farmer _returnvalue)
  (bind _asbp_npc (Utilities|Casting|CastToBP_NPC _returnvalue))
  (Default|EventGotoTarget _asbp_npc))