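; Farmable tree plot that grows fruit while watered and harvests it into the GM_Farmer totals.
; Interacting opens a paused tree selection menu when unplanted, otherwise collects the fruit by type.
; Incoming damage acts as watering, and a looping timer converts water into fruit, refreshing the info widget.
; Each tree persists in an SG_Tree save slot named after the actor, written on planting and growth ticks but not on harvest.
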(event Custom|CustomEvent
  (bind _returnvalue (Game|GetPlayerController 0))
  (bind _returnvalue_2 (UserInterface|CreateWidget "/Game/Blueprınts/Widget_Blueprints/WB_Trees_Selection.WB_Trees_Selection_C"))
  (UserInterface|Viewport|AddtoViewport _returnvalue_2 0)
  (Variables|/Script/Engine.PlayerController|SetbShowMouseCursor _returnvalue true)
  (Input|SetInputModeUIOnly _returnvalue 0 "DoNotLock" false)
  (Game|SetGamePaused true))

(event Custom|CustomEvent_0
  (params (NewMesh :type Static%20Mesh%20Object%20Reference))
  (bind _savegame (Variables|Default|GetSaVEgAME))
  (Components|StaticMesh|SetStaticMesh (Variables|Default|GetTree) NewMesh)
  (Variables|Default|SetIsSellected? true)
  (CallFunction|EventSendInfoTOWidget)
  (SaveGame|DoesSaveGameExist (Variables|Default|GetSave%20Name))
  (if true
    (Variables|/Game/Blueprınts/SG_Tree.SG_Tree_C|SetFruit%20Icon _savegame (Variables|Default|GetFruit%20Icon))
    (Variables|/Game/Blueprınts/SG_Tree.SG_Tree_C|SetIsSellected? _savegame (Variables|Default|GetIsSellected?))
    (Variables|/Game/Blueprınts/SG_Tree.SG_Tree_C|SetTreeStatic _savegame (Variables|Default|GetTreeStatic))
    (Variables|/Game/Blueprınts/SG_Tree.SG_Tree_C|SetFruit _savegame (Variables|Default|GetFruit))
    (SaveGame|SaveGametoSlot _savegame (Variables|Default|GetSave%20Name))
    (Utilities|Time|SetTimerbyFunctionName 0 "Function_Water" 5.0 true)))

(event Custom|Event_SendInfoToWidget
  (bind _returnvalue (UserInterface|CreateWidget "/Game/Blueprınts/Widget_Blueprints/WB_TreeInfo.WB_TreeInfo_C" 0 (Variables|Default|GetWaterAmount) (Variables|Default|GetFruıt%20Amount) (Variables|Default|GetFruit%20Icon)))
  (UserInterface|SetWidget (Variables|Default|GetWidget) _returnvalue))

(event EventBeginPlay
  (bind _asgm_farmer (Utilities|Casting|CastToGM_Farmer (Game|GetGameMode)))
  (Variables|Default|SetAs%20GM%20Farmer _asgm_farmer)
  (Variables|Default|SetSave%20Name (Utilities|GetObjectName self))
  (bind _returnvalue (SaveGame|DoesSaveGameExist (Variables|Default|GetSave%20Name)))
  (if _returnvalue
    (bind _returnvalue_2 (SaveGame|LoadGamefromSlot (Variables|Default|GetSave%20Name)))
    (bind _assg_tree (Utilities|Casting|CastToSG_Tree _returnvalue_2))
    (Variables|Default|SetSaVEgAME _assg_tree)
    (Variables|Default|SetIsSellected? (Variables|/Game/Blueprınts/SG_Tree.SG_Tree_C|GetIsSellected? _assg_tree))
    (Variables|Default|SetFruit (Variables|/Game/Blueprınts/SG_Tree.SG_Tree_C|GetFruit _assg_tree))
    (bind _output_get (Variables|Default|SetTreeStatic (Variables|/Game/Blueprınts/SG_Tree.SG_Tree_C|GetTreeStatic _assg_tree)))
    (Variables|Default|SetFruit%20Icon (Variables|/Game/Blueprınts/SG_Tree.SG_Tree_C|GetFruit%20Icon _assg_tree))
    (Variables|Default|SetWaterAmount (Variables|/Game/Blueprınts/SG_Tree.SG_Tree_C|GetWateramount _assg_tree))
    (Variables|Default|SetFruıt%20Amount (Variables|/Game/Blueprınts/SG_Tree.SG_Tree_C|GetFruitamount _assg_tree))
    (Components|StaticMesh|SetStaticMesh (Variables|Default|GetTree) _output_get)
    (CallFunction|EventSendInfotoWidget)
    (Utilities|Time|SetTimerbyFunctionName 0 "Function_Water" 5.0 true)
    (else
      (bind _returnvalue_3 (SaveGame|CreateSaveGameObject "/Game/Blueprınts/SG_Tree.SG_Tree_C"))
      (Variables|Default|SetSaVEgAME _returnvalue_3))))

(event Collision|EventActorBeginOverlap
  (params (OtherActor :type Actor%20Object%20Reference)))

(event EventTick
  (params (DeltaSeconds :type Float%20%28single-precision%29)))

(event EventFarmInteraction
  (if (Variables|Default|GetIsSellected?)
    (CallFunction|FunctionAddFruit)
    (else
      (CallFunction|CustomEvent))))

(event Game|Damage|EventAnyDamage
  (params (Damage :type Float%20%28single-precision%29) (DamageType :type Damage%20Type%20Object%20Reference) (InstigatedBy :type Controller%20Object%20Reference) (DamageCauser :type Actor%20Object%20Reference))
  (if (Variables|Default|GetIsSellected?)
    (Variables|Default|SetWaterAmount (Math|Float|Clamp(Float) (+ Damage (Variables|Default|GetWaterAmount)) 0.0 1e+02))
    (CallFunction|EventSendInfotoWidget)))

(event EventFunctionSpawnTree
  (params (Tree :type Static%20Mesh%20Object%20Reference) (Fruit :type Name :default "None") (Fruit_Icon :type Texture%202D%20Object%20Reference))
  (Variables|Default|SetFruit Fruit)
  (bind _output_get (Variables|Default|SetTreeStatic Tree))
  (Variables|Default|SetFruit%20Icon Fruit_Icon)
  (CallFunction|CustomEvent0 _output_get))

(fn ConstructionScript)

(fn FunctionWater
  (bind _savegame (Variables|Default|GetSaVEgAME))
  (if (> (Variables|Default|GetWaterAmount) 0.0)
    (Variables|Default|SetWaterAmount (Math|Float|Clamp(Float) (- (Variables|Default|GetWaterAmount) 2.5) 0.0 1e+02))
    (Variables|Default|SetFruıt%20Amount (Math|Float|Clamp(Float) (+ (Variables|Default|GetFruıt%20Amount) 5.0) 0.0 2e+02))
    (CallFunction|EventSendInfotoWidget)
    (bind _returnvalue (SaveGame|DoesSaveGameExist (Variables|Default|GetSave%20Name)))
    (if _returnvalue
      (Variables|/Game/Blueprınts/SG_Tree.SG_Tree_C|SetWateramount _savegame (Variables|Default|GetWaterAmount))
      (Variables|/Game/Blueprınts/SG_Tree.SG_Tree_C|SetFruitamount _savegame (Variables|Default|GetFruıt%20Amount))
      (SaveGame|SaveGametoSlot _savegame (Variables|Default|GetSave%20Name)))))

(fn FunctionAddFruit
  (bind _as_gm_farmer (Variables|Default|GetAs%20GM%20Farmer))
  (bind _as_gm_farmer_2 (Variables|Default|GetAs%20GM%20Farmer))
  (bind _as_gm_farmer_3 (Variables|Default|GetAs%20GM%20Farmer))
  (bind _as_gm_farmer_4 (Variables|Default|GetAs%20GM%20Farmer))
  (bind _as_gm_farmer_5 (Variables|Default|GetAs%20GM%20Farmer))
  (if (> (Variables|Default|GetFruıt%20Amount) 0.0)
    (if (== (Variables|Default|GetFruit) "Apple")
      (Variables|/Game/Blueprınts/Character/GM_Farmer.GM_Farmer_C|SetCurrentAppleAmount _as_gm_farmer_4 (+ (Variables|/Game/Blueprınts/Character/GM_Farmer.GM_Farmer_C|GetCurrentAppleAmount _as_gm_farmer_4) (Variables|Default|GetFruıt%20Amount)))
      (Variables|Default|SetFruıt%20Amount 0.0)
      (CallFunction|EventSendInfotoWidget)
      (elif (== (Variables|Default|GetFruit) "Orange")
        (Variables|/Game/Blueprınts/Character/GM_Farmer.GM_Farmer_C|SetCurrentOrangeAmount _as_gm_farmer_5 (+ (Variables|/Game/Blueprınts/Character/GM_Farmer.GM_Farmer_C|GetCurrentOrangeAmount _as_gm_farmer_5) (Variables|Default|GetFruıt%20Amount)))
        (Variables|Default|SetFruıt%20Amount 0.0)
        (CallFunction|EventSendInfotoWidget)
        (elif (== (Variables|Default|GetFruit) "Pear")
          (Variables|/Game/Blueprınts/Character/GM_Farmer.GM_Farmer_C|SetCurrentPearAmount _as_gm_farmer (+ (Variables|/Game/Blueprınts/Character/GM_Farmer.GM_Farmer_C|GetCurrentPearAmount _as_gm_farmer) (Variables|Default|GetFruıt%20Amount)))
          (Variables|Default|SetFruıt%20Amount 0.0)
          (CallFunction|EventSendInfotoWidget)
          (elif (== (Variables|Default|GetFruit) "Peach")
            (Variables|/Game/Blueprınts/Character/GM_Farmer.GM_Farmer_C|SetCurrentPeachAmount _as_gm_farmer_2 (+ (Variables|/Game/Blueprınts/Character/GM_Farmer.GM_Farmer_C|GetCurrentPeachAmount _as_gm_farmer_2) (Variables|Default|GetFruıt%20Amount)))
            (Variables|Default|SetFruıt%20Amount 0.0)
            (CallFunction|EventSendInfotoWidget)
            (elif (== (Variables|Default|GetFruit) "Pomagranate")
              (Variables|/Game/Blueprınts/Character/GM_Farmer.GM_Farmer_C|SetCurrentPomagranteAmount _as_gm_farmer_3 (+ (Variables|/Game/Blueprınts/Character/GM_Farmer.GM_Farmer_C|GetCurrentPomagranteAmount _as_gm_farmer_3) (Variables|Default|GetFruıt%20Amount)))
              (Variables|Default|SetFruıt%20Amount 0.0)
              (CallFunction|EventSendInfotoWidget))))))))