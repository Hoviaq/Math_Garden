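; BP_Screen is an in-world computer screen actor that opens a computer UI for the player in the farming game.
; On BeginPlay it hands its SpawnerRef to the GM_Farmer game mode as that mode's Spawner.
; Its FarmInteraction event creates a WB_ComputerScreen widget with TableRef, adds it to the viewport, shows the mouse cursor and switches input to UI only.
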(event EventBeginPlay
  (bind _asgm_farmer (Utilities|Casting|CastToGM_Farmer (Game|GetGameMode)))
  (Variables|/Game/Blueprınts/Character/GM_Farmer.GM_Farmer_C|SetSpawner _asgm_farmer (Variables|Default|GetSpawner_Ref)))

(event Collision|EventActorBeginOverlap
  (params (OtherActor :type Actor%20Object%20Reference)))

(event EventTick
  (params (DeltaSeconds :type Float%20%28single-precision%29)))

(event EventFarmInteraction
  (bind _returnvalue (Game|GetPlayerController 0))
  (bind _returnvalue_2 (UserInterface|CreateWidget "/Game/Blueprınts/Widget_Blueprints/WB_ComputerScreen.WB_ComputerScreen_C" 0 (Variables|Default|GetTable_Ref)))
  (UserInterface|Viewport|AddtoViewport _returnvalue_2 0)
  (Variables|/Script/Engine.PlayerController|SetbShowMouseCursor _returnvalue true)
  (Input|SetInputModeUIOnly _returnvalue 0 "DoNotLock" false))

(fn ConstructionScript)